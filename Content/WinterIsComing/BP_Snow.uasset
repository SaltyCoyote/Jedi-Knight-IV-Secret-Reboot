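; BP_Snow is an advancing winter hazard that damages BP_MasterUnit actors it covers.
; Every five seconds, Tick steps it along negative Y by a random amount scaled by frame time.
; A second DoOnce damages units overlapping WinterArea about once per second, destroying those without health.
; That DoOnce resets only inside the overlap loop, so damage stops permanently after an empty check.
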(event `self.ReceiveTick`
  (params (DeltaSeconds :type "Float (single-precision)"))
  (bind (_returnvalue_x _returnvalue_y _returnvalue_z) (`KismetMathLibrary.BreakVector` (`SceneComponent.K2_GetComponentLocation` (`self.DefaultSceneRoot`))))
  (`|ExecutionSequence`
    (:`then_0`
      ;[1 1 1] Snow Progress Condition
      (`/Engine/EditorBlueprintResources/StandardMacros.DoOnce` false :!label _label
        (:`Completed`
          (set `self.CanSnowProgress?` true)
          (`KismetSystemLibrary.Delay` 5.0)
          (goto _label :!via `Reset`))))
    (:`then_1`
      ;[1 1 1] SnowProgression
      (if (`self.CanSnowProgress?`)
        (`SceneComponent.K2_SetWorldLocation` (`self.DefaultSceneRoot`) (`KismetMathLibrary.MakeVector` _returnvalue_x (- _returnvalue_y (* DeltaSeconds (`KismetMathLibrary.RandomFloatInRange` 1000.0 10000.0))) _returnvalue_z) false false)
        (set `self.CanSnowProgress?` false)))
    (:`then_2`
      ;[1 1 1] Damage Player OnOverlap
      (`/Engine/EditorBlueprintResources/StandardMacros.DoOnce` false :!label _label_2
        (:`Completed`
          (for _array_element (`PrimitiveComponent.GetOverlappingActors` (`self.WinterArea`) "/Game/RTS_Builder_Template/Blueprints/UnitActors/BP_MasterUnit.BP_MasterUnit_C")
            (bind _asbp_master_unit (cast `/Game/RTS_Builder_Template/Blueprints/UnitActors/BP_MasterUnit` _array_element))
            (`/Game/RTS_Builder_Template/Blueprints/UnitActors/BP_MasterUnit.Deduct Health` _asbp_master_unit 0.5 null)
            (if (<= (`/Game/RTS_Builder_Template/Blueprints/UnitActors/BP_MasterUnit.Current Health` _asbp_master_unit) 0.0)
              (`self.K2_DestroyActor` _asbp_master_unit))
            (`KismetSystemLibrary.Delay` 1.0)
            (goto _label_2 :!via `Reset`)))))))

(fn `UserConstructionScript`)