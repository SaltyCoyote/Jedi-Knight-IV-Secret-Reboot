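; BP_Wolf is an animal actor that runs and bites, damaging BP_MasterUnit actors.
; Run raises walk speed, while Attack plays bite animation and sound, applies damage, then restores the animation blueprint.
; The Attacking flag acts as a ready gate, cleared during the delayed cooldown.
; Damage requires an active overlap, tracked by a boolean, and casts the last begin-overlap actor before deducting health through a DoOnce.
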(event `Run`
  ;[1 1 1] Running
  (set `CharacterMovementComponent.MaxWalkSpeed` 500.0 (`self.CharacterMovement`)))

(event `Attack`
  ;[1 1 1] Attack
  (if (`self.Attacking`)
    (`SkeletalMeshComponent.PlayAnimation` (`self.Mesh`) "/Game/AnimalVarietyPack/Wolf/Animations/ANIM_Wolf_Bite.ANIM_Wolf_Bite" false)
    (`GameplayStatics.PlaySoundAtLocation` "/Game/Wav/Feedbacks/Animals/Wolf/Wolf_Attack.Wolf_Attack" (`self.K2_GetActorLocation`) (struct) 1.0 1.0 0.0 null null null)
    (`self.AttackDamage`)
    (set `self.Attacking` false)
    (`KismetSystemLibrary.Delay` 0.66)
    (`SkeletalMeshComponent.SetAnimationMode` (`self.Mesh`) "AnimationBlueprint")
    (`KismetSystemLibrary.Delay` 1.0)
    (set `self.Attacking` true)))

(event `AttackDamage`
  ;[1 1 1] Attack Damage
  (if (`self.IsOverlapingPlayer`)
    (bind _asbp_master_unit (cast `/Game/RTS_Builder_Template/Blueprints/UnitActors/BP_MasterUnit` (stale `self.ReceiveActorBeginOverlap` OtherActor)))
    (`/Engine/EditorBlueprintResources/StandardMacros.IsValid` _asbp_master_unit
      (:`Is Valid`
        (`/Engine/EditorBlueprintResources/StandardMacros.DoOnce` false :!label _label
          (:`Completed`
            (if (`self.Attacking`)
              (`/Game/RTS_Builder_Template/Blueprints/UnitActors/BP_MasterUnit.Deduct Health` _asbp_master_unit 10.0 null)
              (goto _label :!via `Reset`)))))
      (:`Is Not Valid`
        (goto _label :!via `Reset`)))))

(event `self.ReceiveActorBeginOverlap`
  (params (OtherActor :type "Actor Object Reference"))
  ;[1 1 1] Attack Damage
  (set `self.IsOverlapingPlayer` true))

(event `self.ReceiveActorEndOverlap`
  (params (OtherActor :type "Actor Object Reference"))
  ;[1 1 1] Attack Damage
  (set `self.IsOverlapingPlayer` false))

(fn `UserConstructionScript`)