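; FireCamp is an RTS campfire actor that consumes the player's wood while any unit stands near it.
; Every tick, a Check event sets a flag from whether its Sphere overlaps any BP_MasterUnit.
; While the flag is set, a DoOnce reset by a one-second Delay subtracts one WoodResource from BP_RTSPawn each second, with no lower limit.
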(event `Check`
  (if (`KismetArrayLibrary.Array_IsValidIndex` (`PrimitiveComponent.GetOverlappingActors` (`self.Sphere`) "/Game/RTS_Builder_Template/Blueprints/UnitActors/BP_MasterUnit.BP_MasterUnit_C"))
    (set `self.isSomeoneHere` true)
    (else
      (set `self.isSomeoneHere` false))))

(event `self.ReceiveTick`
  (params (DeltaSeconds :type "Float (single-precision)"))
  (bind _asbp_rtspawn (cast `/Game/RTS_Builder_Template/Blueprints/Player/BP_RTSPawn` (`GameplayStatics.GetPlayerPawn` 0) :!pure true))
  (`self.Check`)
  (if (`self.isSomeoneHere`)
    (`/Engine/EditorBlueprintResources/StandardMacros.DoOnce` false :!label _label
      (:`Completed`
        (set `/Game/RTS_Builder_Template/Blueprints/Player/BP_RTSPawn.Wood Resource` (- (`/Game/RTS_Builder_Template/Blueprints/Player/BP_RTSPawn.Wood Resource` _asbp_rtspawn) 1) _asbp_rtspawn)
        (`KismetSystemLibrary.Delay` 1.0)
        (goto _label :!via `Reset`)))))

(fn `UserConstructionScript`)