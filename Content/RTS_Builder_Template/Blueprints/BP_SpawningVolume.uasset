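; BP_SpawningVolume scatters resource actors on the landscape within its bounds, on begin play, on a looping timer, or both.
; SpawnResources picks random points in the bounds, box-traces vertically for ground, and spawns the given class only where it hits Landscape.
; The maximum count is checked only at begin play; timer spawns neither check nor increment the total.
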(event `self.ReceiveBeginPlay`
  ;[1 1 1] Spawn on begin play, timer or both
  (if (and (`self.Spawn On Begin Play`) (< (`self.Total Number Spawned`) (`self.Max Number Spawned`)))
    (`self.Spawn Resources` (`self.Spawn Number`) (`self.Spawn Resource`))
    (set `self.Total Number Spawned` (+ (`self.Spawn Number`) (`self.Total Number Spawned`))))
  (if (and (`self.Spawn On Timer`) (< (`self.Total Number Spawned`) (`self.Max Number Spawned`)))
    (`KismetSystemLibrary.K2_SetTimerDelegate` (delegate `Spawn Resources On Timer`) (`self.Timer Length`) true)))

(event `Spawn Resources On Timer`
  ;[1 1 1] Spawn on begin play, timer or both
  (`self.Spawn Resources` (`self.Spawn Number`) (`self.Spawn Resource`)))

(fn `Spawn Resources`
  (params (`Spawn Number` :type Integer) (`Spawn Resource` :type "/Game/RTS_Builder_Template/Blueprints/ResourceActors/BP_MasterResource Class Reference"))
  (locals (`L Spawn Number` :type Integer) (`L Spawn Resource` :type "/Game/RTS_Builder_Template/Blueprints/ResourceActors/BP_MasterResource Class Reference") (`L X Random Float` :type "Float (double-precision)") (`L Y Random Float` :type "Float (double-precision)"))
  (bind (_origin _boxextent) (`self.GetActorBounds` false))
  (bind _x (.x _boxextent))
  (bind _y (.y _boxextent))
  (bind _returnvalue (+ _origin (`KismetMathLibrary.MakeVector` (`KismetMathLibrary.RandomFloatInRange` (- _x (* _x 2.0)) _x) (`KismetMathLibrary.RandomFloatInRange` (- _y (* _y 2.0)) _y) (.z _origin))))
  ;[1 1 1] Set local variables
  (set `local.L Spawn Number` `Spawn Number`)
  (set `local.L Spawn Resource` `Spawn Resource`)
  ;[1 1 1] Loop for the number of actors to spawn
  (for _ (range 1 (+ (`local.L Spawn Number`) 1))
    ;[1 1 1] Set random floats
    (set `local.L X Random Float` (`KismetMathLibrary.RandomFloatInRange` 0.0 2.0))
    (set `local.L Y Random Float` (`KismetMathLibrary.RandomFloatInRange` 0.0 2.0))
    ;[1 1 1] Box trace to check for the ground
    (bind _outhit (`KismetSystemLibrary.BoxTraceSingle` (+ _returnvalue (0.0 0.0 1000.0)) (- _returnvalue (0.0 0.0 1000.0)) (100.0 100.0 50.0) (struct) "TraceTypeQuery1"))
    (bind (_bblockinghit _binitialoverlap _time _distance _location _impactpoint _normal _impactnormal _physmat _hitactor) (`GameplayStatics.BreakHitResult` _outhit))
    ;[1 1 1] Spawn actor at random location
    (if (== (`GameplayStatics.GetObjectClass` _hitactor) "/Script/Landscape.Landscape")
      (`|SpawnActorFromClass` (`local.L Spawn Resource`) (`KismetMathLibrary.Conv_VectorToTransform` _location) "AlwaysSpawn" "OverrideRootScale" null null))))

(fn `UserConstructionScript`)