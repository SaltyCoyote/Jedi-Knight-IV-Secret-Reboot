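; Base resource actor for the RTS builder, holding an amount that DeductResources lowers, returning false once it hits zero.
; Construction fills it to full, optionally randomizes mesh scale and yaw, and sizes the selection ring.
; Tick compares itself to the RTS pawn's saved hit actor, using paired DoOnce gates to add or remove a duplicate-mesh outline with a dynamic material.
; The CanOutline check is disconnected.
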(event `self.ReceiveTick`
  (params (DeltaSeconds :type "Float (single-precision)"))
  (if (== (`/Game/RTS_Builder_Template/Blueprints/Player/BP_RTSPawn.ActorHitSaved` (cast `/Game/RTS_Builder_Template/Blueprints/Player/BP_RTSPawn` (`GameplayStatics.GetPlayerPawn` 0) :!pure true)) self)
    (`/Engine/EditorBlueprintResources/StandardMacros.DoOnce` false :!label _label
      (:`Completed`
        (`self.CreateOutline`)
        (goto _label_2 :!via `Reset`)))
    (else
      (`/Engine/EditorBlueprintResources/StandardMacros.DoOnce` false :!label _label_2
        (:`Completed`
          (`self.DeleteOutline`)
          (goto _label :!via `Reset`))))))

(fn `CreateOutline`
  (bind _resourcemesh (`self.ResourceMesh`))
  (if (not (`self.HasOutline`))
    (bind _returnvalue (`AddComponent|NODE_AddStaticMeshComponent-0` :`bManualAttachment` true :`RelativeTransform` (`SceneComponent.K2_GetComponentToWorld` _resourcemesh)))
    (bind _output_get (set `self.OutlineMesh` _returnvalue))
    (`StaticMeshComponent.SetStaticMesh` _output_get (`StaticMeshComponent.StaticMesh` _resourcemesh))
    (bind _returnvalue_2 (`PrimitiveComponent.CreateDynamicMaterialInstance` (`self.OutlineMesh`) 0 "/Game/RTS_Builder_Template/OutlineMaterials/Outline_Inst.Outline_Inst" "None"))
    (`MaterialInstanceDynamic.SetVectorParameterValue` _returnvalue_2 "Color" (struct :`R` 1.0 :`G` 1.0 :`B` 1.0))
    (`MaterialInstanceDynamic.SetScalarParameterValue` _returnvalue_2 "Scale" 20.0)
    (set `self.HasOutline` true)))

(fn `Deduct Resources`
  (params (`Deduct Amount` :type Integer))
  (returns (`Resources Remaining` :type Boolean))
  ;[1 1 1] Deduct the resources from this resource
  (if (> (`self.Current Resources`) `Deduct Amount`)
    (set `self.Current Resources` (- (`self.Current Resources`) `Deduct Amount`))
    (return true)
    (else
      (set `self.Current Resources` 0)
      (return false))))

(fn `DeleteOutline`
  (bind _outlinemesh (`self.OutlineMesh`))
  (if (`self.HasOutline`)
    (`/Engine/EditorBlueprintResources/StandardMacros.IsValid` _outlinemesh
      (:`Is Valid`
        (`ActorComponent.K2_DestroyComponent` _outlinemesh)
        (set `self.HasOutline` false)
        (`SceneComponent.SetVisibility` (`self.ResourceMesh`) true false)))))

(fn `UserConstructionScript`
  (bind _returnvalue (`KismetMathLibrary.RandomFloatInRange` (`self.Min Mesh Size`) (`self.Max Mesh Size`)))
  ;[1 1 1] Set Resources
  (set `self.Current Resources` (`self.Full Resources`))
  ;[1 1 1] If True Use Random Size
  (if (`self.Use Random Size`)
    ;[1 1 1] Set 3D World Size
    (`SceneComponent.SetWorldScale3D` (`self.ResourceMesh`) (`KismetMathLibrary.MakeVector` _returnvalue _returnvalue _returnvalue)))
  ;[1 1 1] If True Use Random Rotation
  (if (`self.Use Random Rotation`)
    ;[1 1 1] Set Random Rotation
    (`SceneComponent.K2_SetWorldRotation` (`self.ResourceMesh`) (`KismetMathLibrary.MakeRotator` 0.0 0.0 (`KismetMathLibrary.RandomFloatInRange` 0.0 365.0)) false false))
  ;[1 1 1] Set the selection ring size
  (`SceneComponent.SetWorldScale3D` (`self.SelectionRing`) (+ (`SceneComponent.K2_GetComponentScale` (`self.ResourceMesh`)) (1.5 1.5 1.5))))