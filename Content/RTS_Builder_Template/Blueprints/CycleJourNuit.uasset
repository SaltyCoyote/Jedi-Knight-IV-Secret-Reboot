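; Day-night cycle actor for the RTS builder template that rotates a directional light and advances a TimeOfDay counter.
; Tick drives a DoOnce that steps the light and counter, then resets after a delay, throttling updates.
; The delay derives from DeltaSeconds and shrinks as CustomTimeDilation rises.
; TimeOfDay wraps to zero on reaching its limit, independently of the light's rotation.
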(event `self.ReceiveTick`
  (params (DeltaSeconds :type "Float (single-precision)"))
  (if (>= (`self.TimeOfDay`) 60.0)
    (set `self.TimeOfDay` 0.0))
  (`/Engine/EditorBlueprintResources/StandardMacros.DoOnce` false :!label _label
    (:`Completed`
      (`SceneComponent.K2_AddLocalRotation` (`self.DirectionalLight`) (struct :`Pitch` 0.05) false false)
      (set `self.TimeOfDay` (+ (`self.TimeOfDay`) 1.0))
      (`KismetSystemLibrary.Delay` (/ (+ DeltaSeconds 0.5) (* (`self.CustomTimeDilation`) 2.0)))
      (goto _label :!via `Reset`))))

(fn `UserConstructionScript`)