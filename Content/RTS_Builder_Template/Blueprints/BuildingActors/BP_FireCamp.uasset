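; BP_FireCamp is a fire camp building actor that drains the player's wood while a BP_DetectionRange actor overlaps it.
; Overlap events set the IsSomeoneHere flag, though any other actor type beginning overlap clears it.
; While the flag is set, Tick uses a DoOnce reset by a Delay to subtract WoodResource on BP_RTSPawn once per second.
; The CheckOverlapping event called from Tick is empty.
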(event `self.ReceiveActorBeginOverlap`
  (params (OtherActor :type "Actor Object Reference"))
  (cast `/Game/RTS_Builder_Template/Blueprints/Others/BP_DetectionRange` OtherActor
    (:`then`
      (set `self.isSomeoneHere` true))
    (:`CastFailed`
      (set `self.isSomeoneHere` false))))

(event `self.ReceiveActorEndOverlap`
  (params (OtherActor :type "Actor Object Reference"))
  (cast `/Game/RTS_Builder_Template/Blueprints/Others/BP_DetectionRange` OtherActor)
  (set `self.isSomeoneHere` false))

(event `CheckOverlapping`)

(event `self.ReceiveTick`
  (params (DeltaSeconds :type "Float (single-precision)"))
  (bind _asbp_rtspawn (cast `/Game/RTS_Builder_Template/Blueprints/Player/BP_RTSPawn` (`GameplayStatics.GetPlayerPawn` 0) :!pure true))
  (`parent.ReceiveTick` DeltaSeconds)
  (`self.CheckOverlapping`)
  (if (`self.isSomeoneHere`)
    (`/Engine/EditorBlueprintResources/StandardMacros.DoOnce` false :!label _label
      (:`Completed`
        (set `/Game/RTS_Builder_Template/Blueprints/Player/BP_RTSPawn.Wood Resource` (- (`/Game/RTS_Builder_Template/Blueprints/Player/BP_RTSPawn.Wood Resource` _asbp_rtspawn) 1) _asbp_rtspawn)
        (`KismetSystemLibrary.Delay` 1.0)
        (goto _label :!via `Reset`)))))

(fn `UserConstructionScript`
  (`parent.UserConstructionScript`))