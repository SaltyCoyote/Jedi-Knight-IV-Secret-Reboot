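; Game mode for the RTS builder template that decides when a match is won or lost.
; Each Tick it counts BP_MasterUnit actors, triggering a loss when none remain and otherwise a win if HasWon is set.
; Both branches pass through a DoOnce, which sits ahead of the HasWon check, so that flag is read only once.
; Either result clears widgets, shows a loading screen and opens the win or lose map after a delay.
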(event `WinGame`
  (`WidgetLayoutLibrary.RemoveAllWidgets`)
  (bind _returnvalue (`|CreateWidget` "/Game/MainMenu/LoadingScreenWidget.LoadingScreenWidget_C"))
  (`UserWidget.AddToViewport` _returnvalue 0)
  (`KismetSystemLibrary.Delay` 3.0)
  (`GameplayStatics.OpenLevel` "WinMap"))

(event `Win/Lose`
  (bind _outactors (`GameplayStatics.GetAllActorsOfClass` "/Game/RTS_Builder_Template/Blueprints/UnitActors/BP_MasterUnit.BP_MasterUnit_C"))
  (if (<= (`KismetArrayLibrary.Array_Length` _outactors) 0)
    (`/Engine/EditorBlueprintResources/StandardMacros.DoOnce` false
      (:`Completed`
        (`self.LoseGame`)))
    (else
      (`/Engine/EditorBlueprintResources/StandardMacros.DoOnce` false
        (:`Completed`
          (if (`self.hasWon`)
            (`self.WinGame`)))))))

(event `LoseGame`
  (`WidgetLayoutLibrary.RemoveAllWidgets`)
  (bind _returnvalue (`|CreateWidget` "/Game/MainMenu/LoadingScreenWidget.LoadingScreenWidget_C"))
  (`UserWidget.AddToViewport` _returnvalue 0)
  (`KismetSystemLibrary.Delay` 3.0)
  (`GameplayStatics.OpenLevel` "LoseMap"))

(event `self.ReceiveTick`
  (params (DeltaSeconds :type "Float (single-precision)"))
  (`self.Win/Lose`))

(fn `UserConstructionScript`)